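; Gravity volume that changes gravity scale, gravity direction and Ninja movement mode on actors overlapping it.
; On begin overlap, it sends interface messages with its configured values, each gated by its own Update flag.
; On end overlap, it resets scale and downward gravity and sends the inverse Ninja movement state, rather than restoring previous values.
; AlwaysResetGravityDirection forces the direction reset on exit even when direction updates are off.
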(event EventBeginPlay)

(event Collision|EventActorBeginOverlap
  (params (OtherActor :type Actor%20Object%20Reference))
  ;[1 1 1] Beginoverlap
  (Utilities|FlowControl|Sequence
    (:then_0
      (if (Variables|Default|GetUpdateGravity%20scale)
        (Class|BPIGravityToggleAble|SetVolumeGravityScaleMultiplier(Message) OtherActor (Variables|Default|GetGravityScale%20Multiplier))))
    (:then_1
      (if (Variables|Default|GetUpdateGravityDirection)
        (Class|BPIGravityToggleAble|SetGravityDirection(Message) OtherActor (Variables|Default|GetGravity%20Direction))))
    (:then_2
      (if (Variables|Default|GetUpdateNinjaMovement)
        (Class|BPIGravityToggleAble|ToggleNinjaMovement(Message) OtherActor (Variables|Default|GetNinjaMovementOn))))))

(event EventTick
  (params (DeltaSeconds :type Float%20%28single-precision%29)))

(event Collision|EventActorEndOverlap
  (params (OtherActor :type Actor%20Object%20Reference))
  ;[1 1 1] EndOverlap
  (Utilities|FlowControl|Sequence
    (:then_0
      (if (Variables|Default|GetUpdateGravity%20scale)
        (Class|BPIGravityToggleAble|SetVolumeGravityScaleMultiplier(Message) OtherActor 1.0)))
    (:then_1
      (if (or (Variables|Default|GetUpdateGravityDirection) (Variables|Default|GetAlways%20reset%20Gravity%20Direction))
        (Class|BPIGravityToggleAble|SetGravityDirection(Message) OtherActor "0,0,-1.000000")))
    (:then_2
      (if (Variables|Default|GetUpdateNinjaMovement)
        (Class|BPIGravityToggleAble|ToggleNinjaMovement(Message) OtherActor (not (Variables|Default|GetNinjaMovementOn)))))))

(fn ConstructionScript)