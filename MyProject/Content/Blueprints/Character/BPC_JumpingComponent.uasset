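; Jump component for NinjaPlayerCharacter_BP that handles multi-jump limits, coyote time and rotation-aware jump launches.
; TryJump counts a grounded or coyote jump as one and others as two, recording a buffer deadline on failure.
; Entering falling opens a retriggerable coyote window that uses up the first jump if it expires.
; StartJump and StopJump call LaunchCharacterRotated, the latter overriding vertical velocity capped at JumpZVelocity.
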(event Custom|StartJump
  (bind _ownercharacter (Variables|Default|GetOwnerCharacter))
  (Class|NinjaCharacter|LaunchCharacterRotated _ownercharacter (Math|Vector|MakeVector 0.0 0.0 (Variables|/Script/Engine.CharacterMovementComponent|GetJumpZVelocity (Variables|/Game/Blueprints/Character/NinjaPlayerCharacter_BP.NinjaPlayerCharacter_BP_C|GetNinjaMovementComponent _ownercharacter))) false false))

(event Custom|StopJump
  (bind _ownercharacter (Variables|Default|GetOwnerCharacter))
  (bind _ninjamovementcomponent (Variables|/Game/Blueprints/Character/NinjaPlayerCharacter_BP.NinjaPlayerCharacter_BP_C|GetNinjaMovementComponent _ownercharacter))
  (Class|NinjaCharacter|LaunchCharacterRotated _ownercharacter (Math|Vector|MakeVector 0.0 0.0 (Math|Float|Clamp(Float) (.z (Math|Transform|TransformDirection (Transformation|GetActorTransform _ownercharacter) (Pawn|Components|CharacterMovement|GetLastUpdateVelocity _ninjamovementcomponent))) -99999.0 (Variables|/Script/Engine.CharacterMovementComponent|GetJumpZVelocity _ninjamovementcomponent))) false true))

(event Custom|OnEnteredFallingState
  (if (== (Variables|Default|GetJumpSinceLanding) 0)
    (Variables|Default|SetCoyoteTimeEnd (+ (Variables|Default|GetCoyoteTime) (Utilities|Time|GetTimeSeconds)))
    (Variables|Default|SetisCoyoteTime true)
    (Utilities|FlowControl|RetriggerableDelay (Variables|Default|GetCoyoteTime))
    (if (Variables|Default|GetisCoyoteTime)
      (Variables|Default|SetJumpSinceLanding 1)
      (Variables|Default|SetisCoyoteTime false))))

(event EventBeginPlay
  (bind _asninja_player_character_bp (Utilities|Casting|CastToNinjaPlayerCharacter_BP (Components|GetOwner)))
  (Variables|Default|SetOwnerCharacter _asninja_player_character_bp)
  (Variables|Default|SetMaxJumps (Variables|/Script/Engine.Character|GetJumpMaxCount (Variables|Default|GetOwnerCharacter)))
  (Variables|/Script/Engine.Character|SetJumpMaxCount (Variables|Default|GetOwnerCharacter) (+ (Variables|/Script/Engine.Character|GetJumpMaxCount (Variables|Default|GetOwnerCharacter)) 1)))

(event EventTick
  (params (DeltaSeconds :type Float%20%28single-precision%29)))

(fn TryJump
  (if (< (Variables|Default|GetJumpSinceLanding) (Variables|Default|GetMaxJumps))
    (Variables|Default|SetJumpSinceLanding (+ (Variables|Default|GetJumpSinceLanding) (select (or (CallFunction|CoyoteTimeon) (AI|Components|NavMovement|IsMovingonGround (Variables|/Script/Engine.Character|GetCharacterMovement (Variables|Default|GetOwnerCharacter)))) 1 2)))
    (Variables|Default|SetisCoyoteTime false)
    (return true)
    (else
      (Variables|Default|SetJumpBufferEndTime (+ (Variables|Default|GetJumpBufferInputTime) (Utilities|Time|GetTimeSeconds)))
      (return false))))

(fn CoyoteTimeon
  (return (and (> (Variables|Default|GetCoyoteTimeEnd) (Utilities|Time|GetTimeSeconds)) (Variables|Default|GetisCoyoteTime))))