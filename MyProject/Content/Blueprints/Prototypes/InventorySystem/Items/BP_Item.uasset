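; BP_Item is a quest item pickup that goes into the player's inventory on overlap.
; BeginPlay toggles the mesh and disables collision until SpawnQuestItems toggles it again, enables collision and marks the item spawned.
; Waypoint events set or clear a child actor marker, showing it only for spawned items after a short delay.
; A successful add to the inventory component notifies the player's quest log quests and destroys the item.
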(event OnComponentBeginOverlap(Sphere)
  (params (OverlappedComponent :type Primitive%20Component%20Object%20Reference) (OtherActor :type Actor%20Object%20Reference) (OtherComp :type Primitive%20Component%20Object%20Reference) (OtherBodyIndex :type Integer) (bFromSweep :type Boolean) (SweepResult :type Hit%20Result%20Structure%20%28by%20ref%29))
  ;[1 1 1] Add item to inventory
  (if (== OtherActor (Game|GetPlayerCharacter 0))
    (bind _success (Default|AddtoInventory (Actor|GetComponentbyClass OtherActor "/Game/Blueprints/Prototypes/InventorySystem/BPC_InventoryComponent.BPC_InventoryComponent_C") (Utilities|Struct|MakeStruct_ItemSlots (Variables|Default|GetItemStructure) 1)))
    (if _success
      (for _array_element (Variables|/Game/Blueprints/Prototypes/QuestSystem/BPC_QuestLog.BPC_QuestLog_C|GetQuests (Variables|Default|GetQuestComponent))
        (Default|CallCollectedItem _array_element self)
        (Actor|DestroyActor)))))

(event EventBeginPlay
  ;[1 1 1] Hide quest items in game
  (bind _asninja_player_character_bp (Utilities|Casting|CastToNinjaPlayerCharacter_BP (Game|GetPlayerCharacter 0)))
  (Variables|Default|SetQuestComponent (Variables|/Game/Blueprints/Character/NinjaPlayerCharacter_BP.NinjaPlayerCharacter_BP_C|GetBPC_QuestLog _asninja_player_character_bp))
  (Rendering|ToggleVisibility (Variables|Default|GetStaticMesh) true)
  (Collision|SetActorEnableCollision false))

(event EventSpawnQuestItems
  ;[1 1 1] Spawn quest items when quest is accepted
  (Rendering|ToggleVisibility (Variables|Default|GetStaticMesh) true)
  (Collision|SetActorEnableCollision true)
  (Variables|Default|SetItemHasSpawned true))

(event EventSetWaypointVisibility
  ;[1 1 1] Spawn / remove waypoints
  (Utilities|FlowControl|Delay 0.2)
  (if (Variables|Default|GetItemHasSpawned)
    (ChildActorComponent|SetChildActorClass (Variables|Default|GetChildActor) "/Game/Blueprints/Prototypes/WaypointSystem/BP_WaypointActor.BP_WaypointActor_C")))

(event EventRemoveWaypoints
  ;[1 1 1] Spawn / remove waypoints
  (ChildActorComponent|SetChildActorClass (Variables|Default|GetChildActor) 0))

(fn ConstructionScript)