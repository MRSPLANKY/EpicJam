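; BP_Car is a prototype car hazard that loops along a target spline and launches the player upward on contact.
; When CanMove is set, it waits a random delay, then a timeline lerps distance along the spline to set location only, restarting on finish.
; A box overlap with any BPI_LaunchAble actor launches player character 0 along that actor's up vector, overriding vertical velocity.
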(event OnComponentBeginOverlap(Box)
  (params (OverlappedComponent :type Primitive%20Component%20Object%20Reference) (OtherActor :type Actor%20Object%20Reference) (OtherComp :type Primitive%20Component%20Object%20Reference) (OtherBodyIndex :type Integer) (bFromSweep :type Boolean) (SweepResult :type Hit%20Result%20Structure%20%28by%20ref%29))
  (if (Utilities|DoesObjectImplementInterface OtherActor "/Game/Blueprints/Character/BPI_LaunchAble.BPI_LaunchAble_C")
    (Character|LaunchCharacter (Game|GetPlayerCharacter 0) (* (Transformation|GetActorUpVector OtherActor) 2e+03) false true)))

(event Custom|Start%20Car%20Movement
  (Utilities|FlowControl|Delay (Math|Random|RandomFloatinRange (Variables|Default|GetDelayTimeMin) (Variables|Default|GetDelayTimeMax)))
  (bind _targetspline (Class|BPISpline|GetSpline(Message) (Variables|Default|GetTargetSpline)))
  (bind _newtrack_0 (Timeline|SplineTimeline PlayFromStart)
    (:Update
      (Transformation|SetActorLocation (Spline|GetLocationatDistanceAlongSpline _targetspline (Math|Float|Lerp 0.0 (Spline|GetSplineLength _targetspline) _newtrack_0) "World") false false))
    (:Finished
      (CallFunction|StartCarMovement))))

(event EventBeginPlay
  (if (Variables|Default|GetCanMove)
    (CallFunction|StartCarMovement)))

(fn ConstructionScript)