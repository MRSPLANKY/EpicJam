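; BPC_QuestLog is a quest log component that stores the player's quests and shows or hides the quest log screen.
; AddQuestToLog adds quests uniquely to the Quests list.
; ToggleQuestLog creates WBP_QuestLogUI, anchors it full-screen on the BP_EpicJamMode HUD canvas and enables the cursor with game-and-UI input.
; Toggling again removes the widget and restores game-only input with the cursor hidden.
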(event EventBeginPlay)

(event EventTick
  (params (DeltaSeconds :type Float%20%28single-precision%29)))

(fn AddQuesttoLog
  (params (Quest :type BP%20Quest%20Master%20Object%20Reference))
  (Utilities|Array|AddUnique (Variables|Default|GetQuests) Quest))

(fn ToggleQuestLog
  (bind _returnvalue (Game|GetPlayerController 0))
  (bind _returnvalue_2 (Game|GetPlayerController 0))
  ;[1 1 1] Display Quest Log
  (bind _questlogui (Variables|Default|GetQuestLogUI)
    (:then
      (Widget|RemovefromParent _questlogui)
      (Variables|Default|SetQuestLogUI 0)
      (Input|SetInputModeGameOnly _returnvalue_2)
      (Variables|/Script/Engine.PlayerController|SetbShowMouseCursor _returnvalue_2 false))
    (:else
      (bind _returnvalue_3 (UserInterface|CreateWidget "/Game/Blueprints/Prototypes/QuestSystem/QuestUI/WBP_QuestLogUI.WBP_QuestLogUI_C"))
      (bind _output_get (Variables|Default|SetQuestLogUI _returnvalue_3))
      (bind _asbp_epic_jam_mode (Utilities|Casting|CastToBP_EpicJamMode (Game|GetGameMode)))
      (bind _returnvalue_4 (Class|CanvasPanel|AddChildtoCanvas (Variables|/Game/Blueprints/BP_EpicJamMode.BP_EpicJamMode_C|GetHUD_Canvas _asbp_epic_jam_mode) _output_get))
      (Class|CanvasPanelSlot|SetAnchors _returnvalue_4 (Utilities|Struct|MakeAnchors "(X=0.000000,Y=0.000000)" "(X=1.000000,Y=1.000000)"))
      (Input|SetInputModeGameandUI _returnvalue (Variables|Default|GetQuestLogUI) "DoNotLock" true)
      (Variables|/Script/Engine.PlayerController|SetbShowMouseCursor _returnvalue true))))