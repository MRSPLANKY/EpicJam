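; Quest actor that tracks location and collection objectives for the player, attached to a quest giver actor.
; On BeginPlay it binds location-reached and item-collected events, completing matching objectives after a target or inventory-quantity check and refreshing the HUD objectives widget.
; It messages the parent actor to update waypoint visibility on collection, or to remove waypoints before destroying itself.
; OrganizeQuest snaps it to the quest giver's location.
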(event EventBeginPlay
  (bind _asninja_player_character_bp (Utilities|Casting|CastToNinjaPlayerCharacter_BP (Game|GetPlayerCharacter 0)))
  (bind _output_get (Variables|Default|SetPlayer _asninja_player_character_bp))
  (Variables|Default|SetPlayerInventory (Variables|/Game/Blueprints/Character/NinjaPlayerCharacter_BP.NinjaPlayerCharacter_BP_C|GetBPC_InventoryComponent _output_get))
  (EventDispatchers|BindEventtoLocationReached (EventDispatchers|CreateEvent :!event CheckLocationObjective))
  (EventDispatchers|BindEventtoCollectedItem (EventDispatchers|CreateEvent :!event CheckCollectionObjective)))

(event EventRemoveWaypoints
  (Class|BPIWaypoint|RemoveWaypoints(Message) (Actor|GetAttachParentActor))
  (Actor|DestroyActor))

(fn ConstructionScript)

(fn OrganizeQuest
  ;[1 1 1] Organize quest to corresponding questgiver in editor
  (Transformation|SetActorLocation (Transformation|GetActorLocation (Actor|GetAttachParentActor)) false false))

(fn CheckLocationObjective
  (params (Location%20Reached :type BP%20Location%20Marker%20Object%20Reference))
  ;[1 1 1] Check if Location reached matches location in objectives
  (for (_array_element _array_index) (Variables|Default|GetObjectives)
    (LocalVariables|SetObjectiveNumber _array_index)
    (if (and (not (.IsComplete (Utilities|Struct|BreakStruct_ObjectiveData _array_element))) (== Location%20Reached (.Target (Utilities|Struct|BreakStruct_ObjectiveData _array_element))))
      (Utilities|Array|SetArrayElem (Variables|Default|GetObjectives) (LocalVariables|GetObjectiveNumber) (Utilities|Struct|MakeStruct_ObjectiveData (.description (Utilities|Array|Get(acopy) (Variables|Default|GetObjectives) (LocalVariables|GetObjectiveNumber))) (.objectivetype (Utilities|Array|Get(acopy) (Variables|Default|GetObjectives) (LocalVariables|GetObjectiveNumber))) (.target (Utilities|Array|Get(acopy) (Variables|Default|GetObjectives) (LocalVariables|GetObjectiveNumber))) (.number (Utilities|Array|Get(acopy) (Variables|Default|GetObjectives) (LocalVariables|GetObjectiveNumber))) true))
      (LocalVariables|SetUpdateUI true)))
  ;[1 1 1] Update Objectives UI if anything changed
  (if (LocalVariables|GetUpdateUI)
    (bind _asbp_epic_jam_mode (Utilities|Casting|CastToBP_EpicJamMode (Game|GetGameMode)))
    (Default|UpdateObjectives (Variables|/Game/Blueprints/Prototypes/QuestSystem/QuestUI/WBP_HUD.WBP_HUD_C|GetWBP_ObjectivesUI (Variables|/Game/Blueprints/BP_EpicJamMode.BP_EpicJamMode_C|GetHUD_Widget _asbp_epic_jam_mode)))))

(fn CheckCollectionObjective
  (params (Item :type BP%20Item%20Object%20Reference))
  ;[1 1 1] Compare items to objective
  (for (_array_element _array_index) (Variables|Default|GetObjectives)
    (LocalVariables|SetObjectiveIndex _array_index)
    (if (== (Utilities|GetClass Item) (Utilities|GetClass (.Target (Utilities|Struct|BreakStruct_ObjectiveData _array_element))))
      (bind _isininventory (Default|InventoryQuery (Variables|Default|GetPlayerInventory) (Utilities|GetClass Item) (.Number (Utilities|Struct|BreakStruct_ObjectiveData _array_element))))
      (if _isininventory
        (Utilities|Array|SetArrayElem (Variables|Default|GetObjectives) (LocalVariables|GetObjectiveIndex) (Utilities|Struct|MakeStruct_ObjectiveData (.description (Utilities|Array|Get(acopy) (Variables|Default|GetObjectives) (LocalVariables|GetObjectiveIndex))) (.objectivetype (Utilities|Array|Get(acopy) (Variables|Default|GetObjectives) (LocalVariables|GetObjectiveIndex))) (.target (Utilities|Array|Get(acopy) (Variables|Default|GetObjectives) (LocalVariables|GetObjectiveIndex))) (.number (Utilities|Array|Get(acopy) (Variables|Default|GetObjectives) (LocalVariables|GetObjectiveIndex))) true (.istimedevent (Utilities|Array|Get(acopy) (Variables|Default|GetObjectives) (LocalVariables|GetObjectiveIndex))) (.secondstocomplete (Utilities|Array|Get(acopy) (Variables|Default|GetObjectives) (LocalVariables|GetObjectiveIndex)))))
        (LocalVariables|SetUpdateUI true)
        (Class|BPIWaypoint|SetWaypointVisibility(Message) (Actor|GetAttachParentActor)))))
  ;[1 1 1] Update Objectives UI if anything changed
  (if (LocalVariables|GetUpdateUI)
    (bind _asbp_epic_jam_mode (Utilities|Casting|CastToBP_EpicJamMode (Game|GetGameMode)))
    (Variables|Default|SetHUDWidget (Variables|/Game/Blueprints/BP_EpicJamMode.BP_EpicJamMode_C|GetHUD_Widget _asbp_epic_jam_mode))
    (Default|UpdateObjectives (Variables|/Game/Blueprints/Prototypes/QuestSystem/QuestUI/WBP_HUD.WBP_HUD_C|GetWBP_ObjectivesUI (Variables|/Game/Blueprints/BP_EpicJamMode.BP_EpicJamMode_C|GetHUD_Widget _asbp_epic_jam_mode)))))

(fn SpawnQuestItems
  (params (Item :type BP%20Item%20Object%20Reference))
  (for _array_element (Variables|Default|GetObjectives)
    (bind _outactors (Actor|GetAllActorsOfClass (Utilities|GetClass (.Target (Utilities|Struct|BreakStruct_ObjectiveData _array_element)))))
    (return _outactors)))