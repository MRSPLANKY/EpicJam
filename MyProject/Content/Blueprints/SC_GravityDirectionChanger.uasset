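; Component that changes the gravity direction of actors overlapping its owner.
; It binds to the owner's begin overlap to send a configured direction through SetGravityDirectionMessage, and optionally to end overlap to restore straight-down gravity.
; A ToggleProperty event applies the configured or straight-down direction to a passed-in target.
; The enter handler also prints the direction.
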(event Custom|CustomEvent_0
  (params (OverlappedActor :type Actor%20Object%20Reference) (OtherActor :type Actor%20Object%20Reference))
  (bind _gravitydirectiononenter (Variables|Default|GetGravityDirectionOnEnter))
  (Development|PrintString (Utilities|String|ToString(Vector) _gravitydirectiononenter))
  (Class|BPIGravityToggleAble|SetGravityDirection(Message) OtherActor _gravitydirectiononenter))

(event Custom|CustomEvent_1
  (params (OverlappedActor :type Actor%20Object%20Reference) (OtherActor :type Actor%20Object%20Reference))
  (Class|BPIGravityToggleAble|SetGravityDirection(Message) OtherActor "0,0,-1.000000"))

(event EventBeginPlay
  (bind _returnvalue (Components|GetOwner))
  (Collision|BindEventtoOnActorBeginOverlap _returnvalue (delegate Custom|CustomEvent_0))
  (if (Variables|Default|GetResetOnLeave)
    (Collision|BindEventtoOnActorEndOverlap _returnvalue (delegate Custom|CustomEvent_1))))

(event EventToggleProperty
  (params (NewParam :type Actor%20Object%20Reference%20%28by%20ref%29) (ToggleOn :type Boolean))
  (Class|BPIGravityToggleAble|SetGravityDirection(Message) NewParam (select ToggleOn (Variables|Default|GetGravityDirectionOnEnter) "0, 0,-1.000000")))