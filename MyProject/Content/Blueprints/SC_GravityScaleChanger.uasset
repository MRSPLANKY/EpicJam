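; SC_GravityScaleChanger is a component that turns its owning actor into a gravity volume, changing the gravity scale multiplier of actors that overlap it.
; On BeginPlay it binds to the owner's overlap events, sending NewGravityScaleMultiplier through an interface message on entry.
; If ResetOnEndOverlap is set, exiting restores the default multiplier.
; A ToggleProperty event applies either value to a given target directly.
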(event Custom|ToggleOn
  (params (OverlappedActor :type Actor%20Object%20Reference) (OtherActor :type Actor%20Object%20Reference))
  (Class|BPIGravityToggleAble|SetVolumeGravityScaleMultiplier(Message) OtherActor (Variables|Default|GetNew%20Gravity%20Scale%20multiplier)))

(event Custom|ToggleOff
  (params (OverlappedActor :type Actor%20Object%20Reference) (OtherActor :type Actor%20Object%20Reference))
  (Class|BPIGravityToggleAble|SetVolumeGravityScaleMultiplier(Message) OtherActor 1.0))

(event EventBeginPlay
  (bind _returnvalue (Components|GetOwner))
  (EventDispatchers|AssignOnActorBeginOverlap _returnvalue (delegate Custom|ToggleOn))
  (if (Variables|Default|GetResetOnEndOverlap)
    (EventDispatchers|AssignOnActorEndOverlap _returnvalue (delegate Custom|ToggleOff))))

(event EventTick
  (params (DeltaSeconds :type Float%20%28single-precision%29)))

(event EventToggleProperty
  (params (NewParam :type Actor%20Object%20Reference%20%28by%20ref%29) (ToggleOn :type Boolean))
  (Class|BPIGravityToggleAble|SetVolumeGravityScaleMultiplier(Message) NewParam (Math|Float|SelectFloat (Variables|Default|GetNew%20Gravity%20Scale%20multiplier) 1.0 ToggleOn)))