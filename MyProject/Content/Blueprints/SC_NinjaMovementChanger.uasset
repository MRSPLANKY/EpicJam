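; SC_NinjaMovementChanger is a component that switches ninja movement on for actors that overlap its owning actor.
; On BeginPlay it binds to the owner's begin-overlap event, which prints a debug name and sends ToggleNinjaMovementMessage(true) to the overlapping actor.
; When ResetOnLeave is set, it also binds end-overlap to send false.
; A separate ToggleProperty event forwards the same message with a given state to a supplied target.
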(event Custom|CustomEvent_0
  (params (OverlappedActor :type Actor%20Object%20Reference) (OtherActor :type Actor%20Object%20Reference))
  (Development|PrintString (Utilities|GetDisplayName self))
  (Class|BPIGravityToggleAble|ToggleNinjaMovement(Message) OtherActor true))

(event Custom|CustomEvent_1
  (params (OverlappedActor :type Actor%20Object%20Reference) (OtherActor :type Actor%20Object%20Reference))
  (Class|BPIGravityToggleAble|ToggleNinjaMovement(Message) OtherActor false))

(event EventTick
  (params (DeltaSeconds :type Float%20%28single-precision%29)))

(event EventToggleProperty
  (params (NewParam :type Actor%20Object%20Reference%20%28by%20ref%29) (ToggleOn :type Boolean))
  (Class|BPIGravityToggleAble|ToggleNinjaMovement(Message) NewParam ToggleOn))

(event EventBeginPlay
  (bind _returnvalue (Components|GetOwner))
  (Collision|BindEventtoOnActorBeginOverlap _returnvalue (delegate Custom|CustomEvent_0))
  (if (Variables|Default|GetResetOnLeave)
    (Collision|BindEventtoOnActorEndOverlap _returnvalue (delegate Custom|CustomEvent_1))))